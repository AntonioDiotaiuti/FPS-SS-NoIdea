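; Progression1 is an overlap-triggered actor that plays a timed audio sequence and sets a first-room progression flag.
; The first overlap by an actor tagged Player sets a one-shot guard, waits briefly, then plays a 2D sound.
; When that sound finishes, its audio-finished delegate calls Activate, which sets FirstRoom and plays another 2D sound.
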(event Custom|Activate
  (Variables|Default|SetFirstRoom true)
  (Audio|SpawnSound2D 0 2.0 1.0 0.0 0))

(event Collision|EventActorBeginOverlap
  (params (OtherActor :type Actor%20Object%20Reference))
  (if (Actor|ActorHasTag OtherActor "Player")
    (if (not (Variables|Default|GetPlayerOverlap))
      (Variables|Default|SetPlayerOverlap true)
      (Utilities|FlowControl|Delay 2.0)
      (bind _returnvalue (Audio|SpawnSound2D 0 2.0 1.0 0.0 0))
      (EventDispatchers|BindEventtoOnAudioFinished _returnvalue (delegate Custom|Activate)))))

(fn ConstructionScript)