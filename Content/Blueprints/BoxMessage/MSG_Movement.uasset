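; MSG_Movement is an overlap-triggered message actor that shows the MS_Movement widget, likely a movement hint, to the player.
; When an actor tagged Player begins overlapping, it creates and stores the widget and adds it to the viewport, only if no valid instance exists.
; End overlap removes the widget from its parent without clearing the reference, so re-entry does not re-add it while that instance remains valid.
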(event Collision|EventActorBeginOverlap
  (params (OtherActor :type Actor%20Object%20Reference))
  (if (Actor|ActorHasTag OtherActor "Player")
    (Utilities|IsValid (Variables|Default|GetMyMovingWidget)
      (:Is%20Not%20Valid
        (bind _returnvalue (UserInterface|CreateWidget "/Game/Blueprints/BoxMessage/MS_Movement.MS_Movement_C"))
        (bind _output_get (Variables|Default|SetMyMovingWidget _returnvalue))
        (UserInterface|Viewport|AddtoViewport _output_get 0)))))

(event Collision|EventActorEndOverlap
  (params (OtherActor :type Actor%20Object%20Reference))
  (bind _mymovingwidget (Variables|Default|GetMyMovingWidget))
  (if (Actor|ActorHasTag OtherActor "Player")
    (Utilities|IsValid _mymovingwidget
      (:Is%20Valid
        (Widget|RemovefromParent _mymovingwidget)))))

(fn ConstructionScript)