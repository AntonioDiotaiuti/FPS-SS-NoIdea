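; BP_door is a double sliding door that opens once its Opendoor event has been called three times.
; A Buttonpressed counter increments on each call, and on reaching three the TL_door timeline plays.
; The timeline lerps the left door's relative X location to -200 while the right door mirrors it in the opposite direction.
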(event Custom|Opendoor
  (bind _buttonpressed (Variables|Default|GetButtonpressed))
  (Math|Integer|IncrementInt _buttonpressed
    (:%20%20
      (if (== _buttonpressed 3)
        (bind _newtrack_0 (Timeline|TL_door Play)
          (:Update
            (Transformation|SetRelativeLocation (Variables|Default|Getleftdoor) (Math|Vector|MakeVector (Math|Float|Lerp 0.0 -2e+02 _newtrack_0) 0.0 0.0) false false)
            (Transformation|SetRelativeLocation (Variables|Default|Getrightdoor) (Math|Vector|MakeVector (* (Math|Float|Lerp 0.0 -2e+02 _newtrack_0) -1.0) 0.0 0.0) false false)))))))

(fn ConstructionScript)