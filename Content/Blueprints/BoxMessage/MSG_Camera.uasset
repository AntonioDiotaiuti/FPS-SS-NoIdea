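; MSG_Camera is a trigger actor that switches on a live camera-feed screen while the player is nearby.
; The screen starts glossy black with the scene capture's per-frame capture disabled.
; On player overlap, delayed sounds play, then capture turns on and the screen swaps to the render camera material.
; When the player leaves, capture stops and the screen returns to black, so the capture only updates while the player is present.
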(event EventBeginPlay
  (Rendering|Material|SetMaterial (Variables|/Script/Engine.StaticMeshActor|GetStaticMeshComponent (Variables|Default|GetSchermo)) 0 "/Game/ModSciInteriors/Materials/MI_GlossyBlack.MI_GlossyBlack")
  (Variables|/Script/Engine.SceneCaptureComponent|SetbCaptureEveryFrame (Variables|/Script/Engine.SceneCapture2D|GetCaptureComponent2D (Variables|Default|GetCamera)) false))

(event Collision|EventActorBeginOverlap
  (params (OtherActor :type Actor%20Object%20Reference))
  (bind _camera (Variables|Default|GetCamera))
  (if (Actor|ActorHasTag OtherActor "Player")
    (Utilities|FlowControl|Delay 0.2)
    (Audio|PlaySound2D "/Game/Audio/u_f1ee7vf7na-blip-131856.u_f1ee7vf7na-blip-131856" 1.0 1.0 0.0 0 0)
    (Audio|PlaySound2D "/Game/Audio/Schermo_FILTER.Schermo_FILTER" 1.0 1.0 0.0 0 0)
    (Utilities|FlowControl|Delay 0.2)
    (Audio|PlaySound2D "/Game/Audio/u_f1ee7vf7na-blip-131856.u_f1ee7vf7na-blip-131856" 1.0 1.0 0.0 0 0)
    (Utilities|IsValid _camera
      (:Is%20Valid
        (Variables|/Script/Engine.SceneCaptureComponent|SetbCaptureEveryFrame (Variables|/Script/Engine.SceneCapture2D|GetCaptureComponent2D _camera) true)
        (Rendering|Material|SetMaterial (Variables|/Script/Engine.StaticMeshActor|GetStaticMeshComponent (Variables|Default|GetSchermo)) 0 "/Game/Blueprints/Gameplay/Render_Cam_Mat.Render_Cam_Mat")))))

(event Collision|EventActorEndOverlap
  (params (OtherActor :type Actor%20Object%20Reference))
  (bind _camera (Variables|Default|GetCamera))
  (if (Actor|ActorHasTag OtherActor "Player")
    (Utilities|IsValid _camera
      (:Is%20Valid
        (Variables|/Script/Engine.SceneCaptureComponent|SetbCaptureEveryFrame (Variables|/Script/Engine.SceneCapture2D|GetCaptureComponent2D _camera) false)
        (Rendering|Material|SetMaterial (Variables|/Script/Engine.StaticMeshActor|GetStaticMeshComponent (Variables|Default|GetSchermo)) 0 "/Game/ModSciInteriors/Materials/MI_GlossyBlack.MI_GlossyBlack")))))

(fn ConstructionScript)