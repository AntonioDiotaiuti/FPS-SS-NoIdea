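; BP_CheckPoint is a checkpoint actor that saves the player's respawn point when a Player-tagged actor overlaps it.
; It records progress only when its Index exceeds the Manager's CheckpointIndex, so earlier checkpoints cannot overwrite later ones.
; It converts its local SpawnPosition to world space, copies SpawnRotation unchanged into RespawnData, clears the FirstSpawn flag and prints a confirmation.
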(event Collision|EventActorBeginOverlap
  (params (OtherActor :type Actor%20Object%20Reference))
  (bind _index (Variables|Default|GetIndex))
  (bind _respawndata (Variables|Default|GetRespawnData))
  (bind _manager (Variables|Default|GetManager))
  (if (Actor|ActorHasTag OtherActor "Player")
    (if (> _index (Variables|/Game/Blueprints/Gameplay/BP_RespawnManager.BP_RespawnManager_C|GetCheckpointIndex _manager))
      (Variables|/Game/Blueprints/Gameplay/BP_RespawnManager.BP_RespawnManager_C|SetCheckpointIndex _manager _index)
      (Variables|/Game/Blueprints/Gameplay/PDA_Checkpoint.PDA_Checkpoint_C|SetSpawnPosition _respawndata (Math|Transform|TransformLocation (Transformation|GetActorTransform) (Variables|Default|GetSpawnPosition)))
      (Variables|/Game/Blueprints/Gameplay/PDA_Checkpoint.PDA_Checkpoint_C|SetSpawnRotation _respawndata (Variables|Default|GetSpawnRotation))
      (Variables|/Game/Blueprints/Gameplay/PDA_Checkpoint.PDA_Checkpoint_C|SetFirstSpawn _respawndata false)
      (Development|PrintText "Checkpoint"))))

(fn ConstructionScript)