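; Enemy Blueprint child, apparently of BP_enemyBase, that provides a ShotgunDrop event for spawning a shotgun pickup.
; The event runs a short downward visibility trace from the actor, ignoring the player pawn, and spawns BP_Pickup_Shotgun at the hit location with random yaw.
; The trace result is used without a hit check, and the construction script only calls the parent.
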(event Custom|ShotgunDrop
  (bind _returnvalue (Transformation|GetActorLocation))
  (bind _outhit (Collision|LineTraceByChannel _returnvalue (- _returnvalue "0.000000,0.000000,200.000000") "TraceTypeQuery1" false (Utilities|Array|MakeArray (Game|Player|GetPlayerPawn 0)) "None"))
  (Game|SpawnActorfromClass "/Game/Blueprints/Gameplay/BP_Pickup_Shotgun.BP_Pickup_Shotgun_C" (Math|Transform|MakeTransform (.Location (Collision|BreakHitResult _outhit)) (Math|Rotator|MakeRotator 0.0 0.0 (Math|Random|RandomFloatinRange 0.0 3.6e+02))) "Undefined" "MultiplyWithRoot" 0 0))

(fn ConstructionScript
  (|CallParentFunction))