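; Health component that tracks current health against a maximum, with damage, reset, percentage query and optional auto-regeneration.
; Damage restarts the regen delay and fires damage or zero-health dispatchers; zero health without LastLife also calls Die on the BP_FirstPersonCharacter owner.
; LastLife absorbs the drop to zero silently; a hit taken at zero clears it and signals zero health without calling Die.
; Tick heals over time once the delay has passed.
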(event EventBeginPlay
  (CallFunction|ResetHealth)
  (Variables|Default|SetelapsedTimeBuffer 0.0))

(event EventTick
  (params (DeltaSeconds :type Float%20%28single-precision%29))
  (Utilities|Damaged
    (:Damaged
      (if (Variables|Regen|GetbAutoRegen)
        (CallFunction|HealDamage DeltaSeconds)))))

(fn GetDamage
  (params (DamageAmount :type Float%20%28double-precision%29))
  (Variables|Default|SetelapsedTimeBuffer 0.0)
  (if (and (== (Variables|Default|GetCurrentHealth) 0.0) (Variables|Default|GetlastLife))
    (Variables|Default|SetlastLife false)
    (Default|CallOnHealtZero)
    (else
      (bind _output_get (Variables|Default|SetCurrentHealth (Math|Float|Clamp(Float) (- (Variables|Default|GetCurrentHealth) (Math|Float|Absolute(Float) DamageAmount)) 0.0 (Variables|Default|GetMaxHealth))))
      (if (== _output_get 0.0)
        (if (not (Variables|Default|GetlastLife))
          (Default|CallOnHealtZero)
          (bind _asbp_first_person_character (Utilities|Casting|CastToBP_FirstPersonCharacter (Components|GetOwner)))
          (Default|Die _asbp_first_person_character))
        (else
          (Default|CallOnGetDamage))))))

(fn ResetHealth
  (Variables|Default|SetCurrentHealth (Variables|Default|GetMaxHealth)))

(fn GetCurrentHealthPerc
  (bind _maxhealth (Variables|Default|GetMaxHealth))
  (if (== _maxhealth 0.0)
    (return 1.0)
    (else
      (return (/ (Variables|Default|GetCurrentHealth) _maxhealth)))))

(fn HealDamage
  (params (ElapsedTime :type Float%20%28double-precision%29))
  (bind _output_get (Variables|Default|SetelapsedTimeBuffer (+ (Variables|Default|GetelapsedTimeBuffer) ElapsedTime)))
  (if (>= _output_get (Variables|Regen|GetelapsedTimeForRegen))
    (Variables|Default|SetCurrentHealth (Math|Float|Clamp(Float) (+ (* ElapsedTime (Variables|Default|GetRegenAmount)) (Variables|Default|GetCurrentHealth)) 0.0 (Variables|Default|GetMaxHealth)))))