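; BP_Collision is an interaction trigger that lights a sequence of lamps and then opens a door.
; Player overlap adds an MS_Interact widget if none is stored, and leaving removes it from the viewport without clearing the reference.
; A one-time Interact event starts AccendiLuci, which re-calls itself on a short delay, swapping each "LuceSequenza"-tagged mesh to an emissive material before calling OpenDoorV on DoorV.
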(event Custom|AccendiLuci
  (Rendering|Material|SetMaterial (Variables|/Script/Engine.StaticMeshActor|GetStaticMeshComponent (Utilities|Array|Get(acopy) (Variables|Default|GetListaLuci) (Variables|Default|Getindice))) 2 "/Game/SciFI_Lite_Assets/Materials/MaterialInstances/MI_Emissive_01.MI_Emissive_01")
  (Math|Integer|IncrementInt (Variables|Default|Getindice)
    (:%20%20
      (Utilities|FlowControl|Delay 0.1)
      (if (< (Variables|Default|Getindice) (Utilities|Array|Length (Variables|Default|GetListaLuci)))
        (CallFunction|AccendiLuci)
        (else
          (Default|OpenDoorV (Variables|Default|GetDoorV)))))))

(event EventBeginPlay
  (bind _outactors (Actor|GetAllActorsOfClasswithTag "/Script/Engine.StaticMeshActor" "LuceSequenza"))
  (Variables|Default|SetListaLuci _outactors))

(event Collision|EventActorBeginOverlap
  (params (OtherActor :type Actor%20Object%20Reference))
  (if (Actor|ActorHasTag OtherActor "Player")
    (Utilities|IsValid (Variables|Default|GetMyMovingWidget)
      (:Is%20Not%20Valid
        (bind _returnvalue (UserInterface|CreateWidget "/Game/Blueprints/BoxMessage/MS_Interact.MS_Interact_C"))
        (bind _output_get (Variables|Default|SetMyMovingWidget _returnvalue))
        (UserInterface|Viewport|AddtoViewport _output_get 0)))))

(event EventInteract
  (Utilities|FlowControl|DoOnce false
    (:Completed
      (CallFunction|AccendiLuci))))

(event Collision|EventActorEndOverlap
  (params (OtherActor :type Actor%20Object%20Reference))
  (bind _mymovingwidget (Variables|Default|GetMyMovingWidget))
  (if (Actor|ActorHasTag OtherActor "Player")
    (Utilities|IsValid _mymovingwidget
      (:Is%20Valid
        (Widget|RemovefromParent _mymovingwidget)))))

(fn ConstructionScript)

(fn OpenDoor)