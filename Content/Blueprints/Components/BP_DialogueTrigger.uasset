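; BP_DialogueTrigger is a one-shot trigger that shows a simple dialogue when an actor tagged Player overlaps it.
; On the first such overlap it plays a camera shutter sound and creates WBP_SimpleDialogue with the TestoDaMostrare text on a high viewport layer.
; The widget is removed after a Durata delay, and the DoOnce gate is never reset.
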(event Collision|EventActorBeginOverlap
  (params (OtherActor :type Actor%20Object%20Reference))
  (if (Actor|ActorHasTag OtherActor "Player")
    (Utilities|FlowControl|DoOnce false
      (:Completed
        (Audio|PlaySound2D "/Engine/VREditor/Sounds/UI/Camera_Shutter.Camera_Shutter" 1.0 1.0 0.0 0 0)
        (bind _returnvalue (UserInterface|CreateWidget "/Game/Blueprints/Components/WBP_SimpleDialogue.WBP_SimpleDialogue_C" (Game|GetPlayerController 0) (Variables|Default|GetTestoDaMostrare)))
        (UserInterface|Viewport|AddtoViewport _returnvalue 999)
        (Utilities|FlowControl|Delay (Variables|Default|GetDurata))
        (Widget|RemovefromParent _returnvalue)))))

(fn ConstructionScript)