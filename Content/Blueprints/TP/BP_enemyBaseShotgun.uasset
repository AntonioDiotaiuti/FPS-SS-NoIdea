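; Base shotgun enemy character that takes damage, can be stunned, and shoots the first-person player.
; Its health component triggers death, which stops the AI controller's brain, while a stun pauses that brain briefly.
; Shots are a single sphere trace from the hand socket along capsule forward, drawn persistently for debug, damaging the player's health component.
; Aim, crouch and death functions raise dispatchers for other systems.
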(event Custom|OnDeath
  (CallFunction|Death))

(event Custom|Stun
  (AI|Logic|StopLogic (Variables|/Script/AIModule.AIController|GetBrainComponent (AI|GetAIController (Pawn|GetController))) "Stunned")
  (Utilities|FlowControl|Delay 5.0)
  (Class|BrainComponent|RestartLogic (Variables|/Script/AIModule.AIController|GetBrainComponent (AI|GetAIController (Pawn|GetController)))))

(event EventOnHit
  (params (Damage :type Float%20%28double-precision%29))
  (Default|GetDamage (Variables|Default|GetBP_HealthComponent) Damage))

(event EventBeginPlay
  (EventDispatchers|BindEventtoOnHealtZero (Variables|Default|GetBP_HealthComponent) (delegate Custom|OnDeath)))

(fn ConstructionScript)

(fn Aim
  (Default|CallOnAim))

(fn StopAim
  (Default|CallOnStopAim))

(fn GetFireStart
  (return (Transformation|GetSocketLocation (Variables|Character|GetMesh) "hand_rSocket") (Math|Vector|GetForwardVector (Variables|Collision|GetCapsuleComponent))))

(fn SphereTrace
  (bind (_position _dir) (CallFunction|GetFireStart))
  (bind _weaponinfo (Variables|Default|GetWeaponInfo))
  (bind _outhit (Collision|SphereTraceByChannel _position (+ _position (* _dir (.range _weaponinfo))) 2e+01 "TraceTypeQuery2" false 0 "Persistent"))
  (bind _asbp_first_person_character (Utilities|Casting|CastToBP_FirstPersonCharacter (.HitActor (Collision|BreakHitResult _outhit))))
  (Utilities|IsValid (Actor|GetComponentbyClass _asbp_first_person_character "/Game/Blueprints/Components/BP_HealthComponent.BP_HealthComponent_C")
    (:Is%20Valid
      (Default|GetDamage (Actor|GetComponentbyClass _asbp_first_person_character "/Game/Blueprints/Components/BP_HealthComponent.BP_HealthComponent_C") (.damage _weaponinfo)))))

(fn Death
  (bind _asbp_enemy_aicontroller (Utilities|Casting|CastToBP_EnemyAIController (AI|GetAIController self)))
  (Default|StopBrain _asbp_enemy_aicontroller)
  (Default|CallOnDeathReached))

(fn CrouchMe
  (if (Class|Character|CanCrouch)
    (Character|Crouch)
    (Default|CallOnCrouch)))

(fn UncrouchMe
  (Character|UnCrouch)
  (Default|CallOnUncrouch))