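; BP_Granade is a grenade projectile that explodes where it hits.
; On a hit it plays a sound at the impact location, spawns BP_RocketExplosion there, hands over its ExplosionDamage value and destroys itself.
; Damage is left to the spawned explosion actor, and a leftover physics-impulse branch never runs.
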(event Collision|EventHit
  (params (MyComp :type Primitive%20Component%20Object%20Reference) (Other :type Actor%20Object%20Reference) (OtherComp :type Primitive%20Component%20Object%20Reference) (bSelfMoved :type Boolean) (HitLocation :type Vector :default "0, 0, 0") (HitNormal :type Vector :default "0, 0, 0") (NormalImpulse :type Vector :default "0, 0, 0") (Hit :type Hit%20Result%20Structure%20%28by%20ref%29))
  (Audio|PlaySoundatLocation 0 HitLocation "0, 0, 0" 1.0 1.0 0.0 0 0 0 0)
  (bind _returnvalue (Game|SpawnActorfromClass "/Game/Blueprints/Components/BP_RocketExplosion.BP_RocketExplosion_C" (Math|Transform|MakeTransform HitLocation) "Undefined" "MultiplyWithRoot" 0 0))
  (Variables|/Game/Blueprints/Components/BP_RocketExplosion.BP_RocketExplosion_C|SetExplosionDamage _returnvalue (Variables|Default|GetExplosionDamage))
  (Actor|DestroyActor))

(fn ConstructionScript)